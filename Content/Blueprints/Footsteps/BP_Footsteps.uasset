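; BP_Footsteps is an animation notify that plays a footstep sound matching the surface beneath the animated mesh's owner.
; On notify, it line-traces down the owner's up axis on the Visibility channel, ignoring the owner.
; A hit's physical surface selects a wood, metal or grass sound, with tile as the default.
; The sound plays at the world origin rather than at the owner or hit point.
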(fn `Received_Notify`
  (params (MeshComp :type "SkeletalMeshComponent Object Reference") (Animation :type "AnimSequenceBase Object Reference") (EventReference :type "AnimNotifyEventReference Structure (by ref)"))
  (returns (ReturnValue :type Boolean))
  (bind _returnvalue (`ActorComponent.GetOwner` MeshComp))
  (bind _returnvalue_2 (`Actor.K2_GetActorLocation` _returnvalue))
  (bind (_outhit _returnvalue_3) (`KismetSystemLibrary.LineTraceSingle` _returnvalue_2 (+ _returnvalue_2 (* (`Actor.GetActorUpVector` _returnvalue) -200)) "TraceTypeQuery1" false (`|MakeArray` _returnvalue)))
  (if _returnvalue_3
    (switch `EPhysicalSurface` (`GameplayStatics.GetSurfaceType` _outhit)
      (:`SurfaceType_Default`
        (`GameplayStatics.PlaySoundAtLocation` "/Game/Blueprints/Footsteps/FootstepSFX/Footsteps_Tile/Footsteps_Tile_Run/Footsteps_Tile_Run_03.Footsteps_Tile_Run_03" (0.0 0.0 0.0) (struct) 1.0 1.0 0.0 null null null null))
      (:`SurfaceType1`
        (`GameplayStatics.PlaySoundAtLocation` "/Game/Blueprints/Footsteps/FootstepSFX/Footsteps_Wood/Footsteps_Wood_Jump/Footsteps_Wood_Jump_Land_01.Footsteps_Wood_Jump_Land_01" (0.0 0.0 0.0) (struct) 1.0 1.0 0.0 null null null null))
      (:`SurfaceType2`
        (`GameplayStatics.PlaySoundAtLocation` "/Game/Blueprints/Footsteps/FootstepSFX/Footsteps_Metal/Footsteps_Metal_Run/Footsteps_MetalV1_Run_08.Footsteps_MetalV1_Run_08" (0.0 0.0 0.0) (struct) 1.0 1.0 0.0 null null null null))
      (:`SurfaceType3`
        (`GameplayStatics.PlaySoundAtLocation` "/Game/Blueprints/Footsteps/FootstepSFX/Footsteps_Grass/Footsteps_Grass_Run/Footsteps_Grass_Run_15.Footsteps_Grass_Run_15" (0.0 0.0 0.0) (struct) 1.0 1.0 0.0 null null null null))))
  (return false))