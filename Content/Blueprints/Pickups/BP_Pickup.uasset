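; BP_Pickup is a health pickup that spins in the world until a third-person character touches it.
; A looping timer set on BeginPlay repeatedly tweens the Pickup component through a half turn with MoveComponentTo, then resets its relative rotation.
; Overlapping the Collision component passes the Health value to BP_ThirdPersonCharacter's UpdateHealth, plays a 2D sound and destroys the pickup.
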(event `self.ReceiveBeginPlay`
  ;[0 1 0.8283] BeginPlay
  (`KismetSystemLibrary.K2_SetTimerDelegate` (delegate `Rotate`) 1.1 true))

(event `Rotate`
  ;[1 0.5313 0] Rotate
  (`KismetSystemLibrary.MoveComponentTo` (`self.Pickup`) (0.0 0.0 0.0) (struct :`Yaw` 180.0) false false 1.0)
  (`SceneComponent.K2_SetRelativeRotation` :`self` (`self.Pickup`)))

(event `self.Collision.OnComponentBeginOverlap`
  (params (OverlappedComponent :type "PrimitiveComponent Object Reference") (OtherActor :type "Actor Object Reference") (OtherComp :type "PrimitiveComponent Object Reference") (OtherBodyIndex :type Integer) (bFromSweep :type Boolean) (SweepResult :type "HitResult Structure (by ref)"))
  ;[0.4319 1 0] Add Health
  (bind _asbp_third_person_character (cast `/Game/ThirdPerson/Blueprints/BP_ThirdPersonCharacter` OtherActor))
  (`/Game/ThirdPerson/Blueprints/BP_ThirdPersonCharacter.UpdateHealth` _asbp_third_person_character (`self.Health`))
  (`GameplayStatics.PlaySound2D` (`self.PickupSFX`) 1.0 1.0 0.0 null null)
  (`self.K2_DestroyActor`))

(fn `UserConstructionScript`)