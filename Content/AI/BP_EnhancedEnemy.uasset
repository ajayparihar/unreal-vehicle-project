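; BP_EnhancedEnemy is an AI enemy that reports sight of the player to its Blackboard.
; When PawnSensing sees a BP_ThirdPersonCharacter, it sets the "IsPlayerSeen?" key to true.
; A retriggerable delay slightly longer than the sensing interval acts as a lost-sight timeout, clearing the key once sightings stop.
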(event `self.PawnSensing.OnSeePawn`
  (params (Pawn :type "Pawn Object Reference"))
  (cast `/Game/ThirdPerson/Blueprints/BP_ThirdPersonCharacter` Pawn)
  (`BlackboardComponent.SetValueAsBool` (`AIBlueprintHelperLibrary.GetBlackboard` (`AIBlueprintHelperLibrary.GetAIController` self)) "IsPlayerSeen?" true)
  (`KismetSystemLibrary.RetriggerableDelay` (+ (`PawnSensingComponent.SensingInterval` (`self.PawnSensing`)) 0.1))
  (`BlackboardComponent.SetValueAsBool` (`AIBlueprintHelperLibrary.GetBlackboard` (`AIBlueprintHelperLibrary.GetAIController` self)) "IsPlayerSeen?" false))

(fn `UserConstructionScript`)